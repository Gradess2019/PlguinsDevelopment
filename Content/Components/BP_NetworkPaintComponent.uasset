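; Networked paint component that lets a player start and finish drawing replicated pictures at the component's world location.
; A server call spawns and initializes a BP_ReplicateablePicture, whose rep handler creates the mesh and starts the drawing timeline, invoked manually on non-dedicated servers.
; Finishing routes through the server to a multicast that stops the timeline, enables picture collision and clears the current picture.
; The rep handler still prints a server/client debug string.
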(event Custom|FinishDrawing_Multicast
  (bind _currentpicture (Variables|Default|GetCurrentPicture))
  (Audio|Components|Audio|Stop (Variables|Default|GetDrawingTimeline))
  (Utilities|IsValid _currentpicture
    (:Is%20Valid
      (Class|Picture|EnableCollision _currentpicture)
      (CallFunction|InvalidateCurrentPicture))))

(event Custom|StartDrawing_Server
  (bind _returnvalue (Game|SpawnActorfromClass "/VRPack/Actors/BP_ReplicateablePicture.BP_ReplicateablePicture_C" (Math|Transform|MakeTransform (Transformation|GetWorldLocation) "0, 0, 0" "1,1,1") "AlwaysSpawn" 0 0))
  (Class|Picture|InitializePicture _returnvalue (Variables|Default|GetPictureSettings))
  (Variables|Default|SetCurrentPicture _returnvalue)
  (if (not (Networking|IsDedicatedServer))
    (Class|PaintComponent|OnRepSetCurrentPicture)))

(event Custom|FinishDrawing_Server
  (CallFunction|FinishDrawingMulticast))

(event Custom|InvalidateCurrentPicture
  (Variables|Default|SetCurrentPicture 0))

(event EventFinishDrawing
  (CallFunction|FinishDrawingServer))

(event EventStartDrawing
  (CallFunction|StartDrawingServer))

(event EventDoRepCurrentPicture
  (Utilities|IsValid (Variables|Default|GetCurrentPicture)
    (:Is%20Valid
      (Class|Picture|CreateNewMesh (Variables|Default|GetCurrentPicture) (Transformation|GetWorldLocation))
      (Components|Timeline|PlayfromStart (Variables|Default|GetDrawingTimeline))
      (Development|PrintString (Utilities|String|SelectString "SERVEEEEEEEER" "CLIIIIIEEEEEEEEENTTTTTTTT" (Networking|IsServer)) true true "(R=1.000000,G=0.000000,B=0.064861,A=1.000000)" 5.0))
    (:Is%20Not%20Valid
      (Default|CallOnFinsihDrawing))))